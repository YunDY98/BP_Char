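; Player character Blueprint with control-rotation-relative movement, mouse look, jumping and two key-triggered melee attack animations played directly on the mesh.
; Every Tick, a short line trace from the camera caches the looked-at actor and prints its LookAt message when the hit actor changes.
; Interact messages that actor and, on a truthy result, prints the first InventoryComponent key.
; The Menu input adds a new PlayerMenu widget to the viewport.
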(event EventBeginPlay)

(event EventTick
  (params (DeltaSeconds :type Float%20%28single-precision%29))
  (CallFunction|InteractTrace))

(event Input|ActionEvents|InputActionInteract
  (params (Key :type Key%20Structure :default "None"))
  (:Pressed
    (bind _lookatactor (Variables|Default|GetLookAtActor)
      (:then
        (bind _success (Class|InteractionInterface|Interactwith(Message) _lookatactor self))
        (if _success
          (bind _keys (Utilities|Map|Keys (Variables|/Game/InventorySystem/InventoryComponent.InventoryComponent_C|GetInventoryContent (Variables|Default|GetInventoryComponent))))
          (Development|PrintString (Utilities|String|ToString(Name) (Utilities|Array|Get(acopy) _keys)))))
      (:else))))

(event Input|ActionEvents|InputActionJump
  (params (Key :type Key%20Structure :default "None"))
  (:Pressed
    (Character|Jump)))

(event Input|ActionEvents|InputActionMenu
  (params (Key :type Key%20Structure :default "None"))
  (:Pressed
    (bind _returnvalue (UserInterface|CreateWidget "/Game/InventorySystem/UI/PlayerMenu.PlayerMenu_C"))
    (bind _output_get (Variables|Default|SetNewVar_1 _returnvalue))
    (UserInterface|Viewport|AddtoViewport _output_get 0)))

(event Input|AxisEvents|InputAxisMoveForward/Backward
  (params (AxisValue :type Float%20%28single-precision%29))
  (Pawn|Input|AddMovementInput (Math|Vector|GetForwardVector (Math|Rotator|MakeRotator 0.0 0.0 (.Yaw (Math|Rotator|BreakRotator (Pawn|GetControlRotation :!class /Script/Engine.Pawn))))) AxisValue false))

(event Input|AxisEvents|InputAxisMoveRight/Left
  (params (AxisValue :type Float%20%28single-precision%29))
  (Pawn|Input|AddMovementInput (Math|Vector|GetRightVector (Math|Rotator|MakeRotator 0.0 0.0 (.Yaw (Math|Rotator|BreakRotator (Pawn|GetControlRotation :!class /Script/Engine.Pawn))))) AxisValue false))

(event Input|AxisEvents|InputAxisLookUp/DownMouse
  (params (AxisValue :type Float%20%28single-precision%29))
  (Pawn|Input|AddControllerPitchInput AxisValue))

(event Input|AxisEvents|InputAxisTurnRight/LeftMouse
  (params (AxisValue :type Float%20%28single-precision%29))
  (Pawn|Input|AddControllerYawInput AxisValue))

(event Input|KeyboardEvents|W
  (params (Key :type Key%20Structure :default "None")))

(event Input|KeyboardEvents|C
  (params (Key :type Key%20Structure :default "None"))
  (:Pressed
    (Components|Animation|PlayAnimation (Variables|Character|GetMesh) "/Game/Characters/BP_Nine9Character/Animation/Standing_Melee_Attack_Downward.Standing_Melee_Attack_Downward" false)))

(event Input|KeyboardEvents|Q
  (params (Key :type Key%20Structure :default "None"))
  (:Pressed
    (Components|Animation|PlayAnimation (Variables|Character|GetMesh) "/Game/Characters/BP_Nine9Character/Animation/Sword_And_Shield_Slash_Anim_mixamo_com.Sword_And_Shield_Slash_Anim_mixamo_com" false)))

(fn ConstructionScript)

(fn InteractTrace
  (bind _returnvalue (Game|GetPlayerCameraManager 0))
  (bind _returnvalue_2 (Transformation|GetActorLocation _returnvalue))
  (bind (_outhit _returnvalue_3) (Collision|LineTraceByChannel _returnvalue_2 (+ _returnvalue_2 (* (Transformation|GetActorForwardVector _returnvalue) 3e+02)) "TraceTypeQuery3" false 0 "None"))
  (if _returnvalue_3
    (if (!= (Variables|Default|GetLookAtActor) (.HitActor (Collision|BreakHitResult _outhit)))
      (bind _output_get (Variables|Default|SetLookAtActor (.HitActor (Collision|BreakHitResult _outhit))))
      (bind _message (Class|InteractionInterface|Lookat(Message) _output_get self))
      (Development|PrintString (Utilities|String|ToString(Text) _message)))
    (else
      (Variables|Default|SetLookAtActor 0))))